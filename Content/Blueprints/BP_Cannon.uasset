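; BP_Cannon is a cannon actor that fires once, after a delay from BeginPlay.
; BeginPlay feeds the Arrow's transform and a LeadingATarget result, taken from its forward vector at zero time scalar, into CannonBallPrep.
; CannonBallPrep spawns an actor with no class set, plus sound and explosion effects, ignoring the target, then a timeline moves the barrel along Y.
; An unconnected CannonExample graph holds a looping BP_CannonBall firing version.
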(event Custom|CustomEvent_2)

(event Custom|CustomEvent)

(event Custom|CustomEvent_1)

(event EventBeginPlay
  (bind _arrow (Variables|Default|GetArrow))
  (bind _returnvalue (Transformation|GetWorldLocation _arrow))
  (bind _returnvalue_2 (Transformation|GetWorldRotation _arrow))
  (Utilities|FlowControl|Delay (Variables|Default|GetDuration))
  (bind _newtargetlocation (CallFunction|LeadingATarget _returnvalue (Math|Rotator|GetRotationXVector _returnvalue_2) 0.0))
  (CallFunction|CannonBallPrep _returnvalue _returnvalue_2 _newtargetlocation)
  (bind _cannonmoves (Timeline|Timeline_0 Play)
    (:Update
      (Transformation|SetRelativeLocation (Variables|Default|GetCannon) (Math|Vector|MakeVector 0.0 _cannonmoves 0.0) false false))))

(fn ConstructionScript)

(fn CannonBallPrep
  (params (SpawnTransform :type Vector) (Spawn%20Rotation :type Rotator) (targetLocation :type Vector))
  (Game|SpawnActorfromClass "/Game/Blueprints/BP_CannonBall.BP_CannonBall_C" (Math|Transform|MakeTransform SpawnTransform Spawn%20Rotation "1.000000,1.000000,1.000000") "Undefined" "MultiplyWithRoot" 0 0)
  (Audio|SpawnSoundatLocation "/Game/Sounds/powerful-cannon-shot-352459.powerful-cannon-shot-352459" SpawnTransform "0, 0, 0" 1.0 1.0 0.0 0 0)
  (Effects|SpawnEmitteratLocation "/Game/StarterContent/Particles/P_Explosion.P_Explosion" SpawnTransform Spawn%20Rotation))

(fn NewFunction
  (params (newMultiplier :type Float%20%28double-precision%29))
  (return 0.0))