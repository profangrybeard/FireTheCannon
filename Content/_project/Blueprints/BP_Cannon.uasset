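; BP_Cannon is a cannon the player can fire while standing inside its FireArea.
; Overlapping FireArea sets CanFire and a cannon reference on the third-person player controller, and leaving clears both.
; FireTheCannon! calls CannonBallPrep to spawn a cannonball, sound and explosion effect at the Arrow, then plays a recoil timeline.
; The computed LeadingATarget value goes unused inside CannonBallPrep, and the looping CannonExample graph never runs.
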(event OnComponentBeginOverlap(FireArea)
  (params (OverlappedComponent :type Primitive%20Component%20Object%20Reference) (OtherActor :type Actor%20Object%20Reference) (OtherComp :type Primitive%20Component%20Object%20Reference) (OtherBodyIndex :type Integer) (bFromSweep :type Boolean) (SweepResult :type Hit%20Result%20Structure%20%28by%20ref%29))
  (bind _asbp_third_person_character (Utilities|Casting|CastToBP_ThirdPersonCharacter OtherActor))
  (bind _asbp_third_person_player_controller (Utilities|Casting|CastToBP_ThirdPersonPlayerController (Pawn|GetController _asbp_third_person_character)))
  (Variables|/Game/ThirdPerson/Blueprints/BP_ThirdPersonPlayerController.BP_ThirdPersonPlayerController_C|SetcanFire _asbp_third_person_player_controller true)
  (Variables|/Game/ThirdPerson/Blueprints/BP_ThirdPersonPlayerController.BP_ThirdPersonPlayerController_C|Setcannon _asbp_third_person_player_controller self))

(event OnComponentEndOverlap(FireArea)
  (params (OverlappedComponent :type Primitive%20Component%20Object%20Reference) (OtherActor :type Actor%20Object%20Reference) (OtherComp :type Primitive%20Component%20Object%20Reference) (OtherBodyIndex :type Integer))
  (bind _asbp_third_person_character (Utilities|Casting|CastToBP_ThirdPersonCharacter OtherActor))
  (bind _asbp_third_person_player_controller (Utilities|Casting|CastToBP_ThirdPersonPlayerController (Pawn|GetController _asbp_third_person_character)))
  (Variables|/Game/ThirdPerson/Blueprints/BP_ThirdPersonPlayerController.BP_ThirdPersonPlayerController_C|SetcanFire _asbp_third_person_player_controller false)
  (Variables|/Game/ThirdPerson/Blueprints/BP_ThirdPersonPlayerController.BP_ThirdPersonPlayerController_C|Setcannon _asbp_third_person_player_controller 0))

(event Custom|CustomEvent_2)

(event Custom|CustomEvent)

(event Custom|FireTheCannon!
  (bind _arrow (Variables|Default|GetArrow))
  (bind _returnvalue (Transformation|GetWorldLocation _arrow))
  (bind _returnvalue_2 (Transformation|GetWorldRotation _arrow))
  (bind _newtargetlocation (CallFunction|LeadingATarget _returnvalue (Math|Rotator|GetRotationXVector _returnvalue_2) 0.0))
  (CallFunction|CannonBallPrep _returnvalue _returnvalue_2 _newtargetlocation)
  (bind _cannonmoves (Timeline|Timeline_0 Play)
    (:Update
      (Transformation|SetRelativeLocation (Variables|Default|GetCannon) (Math|Vector|MakeVector 0.0 _cannonmoves 0.0) false false))))

(event Custom|CustomEvent_1)

(fn ConstructionScript)

(fn CannonBallPrep
  (params (SpawnTransform :type Vector) (Spawn%20Rotation :type Rotator) (targetLocation :type Vector))
  (Game|SpawnActorfromClass "/Game/_project/Blueprints/BP_CannonBall.BP_CannonBall_C" (Math|Transform|MakeTransform SpawnTransform Spawn%20Rotation "1.000000,1.000000,1.000000") "Undefined" "MultiplyWithRoot" 0 0)
  (Audio|SpawnSoundatLocation "/Game/_project/Sounds/powerful-cannon-shot-352459.powerful-cannon-shot-352459" SpawnTransform "0, 0, 0" 1.0 1.0 0.0 0 0)
  (Effects|SpawnEmitteratLocation "/Game/StarterContent/Particles/P_Explosion.P_Explosion" SpawnTransform Spawn%20Rotation))

(fn NewFunction
  (params (newMultiplier :type Float%20%28double-precision%29))
  (return 0.0))