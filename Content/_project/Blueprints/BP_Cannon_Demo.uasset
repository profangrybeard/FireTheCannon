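; Demo cannon actor that fires automatically from BeginPlay and can be turned with a key press.
; After a FireRate delay it spawns a BP_CannonBall_Demo at the Arrow component, with shot sound and explosion emitter.
; A Recoil timeline then moves the Cannon component along local Y, and its Update output loops back into the delay to repeat firing.
; Pressing 1 sets actor yaw to the cannon's world yaw plus 15 degrees.
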(event EventBeginPlay
  (bind _arrow (Variables|Default|GetArrow))
  (bind _returnvalue (Transformation|GetWorldLocation _arrow))
  (Utilities|FlowControl|Delay (Variables|CannonProperties|GetFireRate) :!label _label)
  (Game|SpawnActorfromClass "/Game/_project/Blueprints/BP_CannonBall_Demo.BP_CannonBall_Demo_C" (Math|Transform|MakeTransform _returnvalue (Transformation|GetWorldRotation _arrow) "1.000000,1.000000,1.000000") "Undefined" "MultiplyWithRoot" 0 0)
  (Audio|SpawnSoundatLocation "/Game/_project/Sounds/powerful-cannon-shot-352459.powerful-cannon-shot-352459" _returnvalue "0, 0, 0" 1.0 1.0 0.0 0 0)
  (Effects|SpawnEmitteratLocation "/Game/StarterContent/Particles/P_Explosion.P_Explosion" _returnvalue)
  (bind _cannon_movement (Timeline|Recoil PlayFromStart)
    (:Update
      (Transformation|SetRelativeLocation (Variables|Default|GetCannon) (Math|Vector|MakeVector 0.0 _cannon_movement 0.0) false false)
      (goto _label))))

(event Collision|EventActorBeginOverlap
  (params (OtherActor :type Actor%20Object%20Reference)))

(event EventTick
  (params (DeltaSeconds :type Float%20%28single-precision%29)))

(event Input|KeyboardEvents|1
  (params (Key :type Key%20Structure))
  (:Pressed
    (Transformation|SetActorRotation (Math|Rotator|MakeRotator 0.0 0.0 (+ (.yaw (Transformation|GetWorldRotation (Variables|Default|GetCannon))) 15.0)))))

(fn ConstructionScript)